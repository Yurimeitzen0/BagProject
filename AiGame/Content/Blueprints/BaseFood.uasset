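; BaseFood is a consumable item actor that restores one of an AI character's stats when used.
; UseItem adds StatRestore to the character's AiStatArray entry at StatIndex, clamped to that stat's minimum and maximum.
; It writes the rebuilt stat struct back with the other fields unchanged, then destroys the food actor.
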(event `/Game/Interfaces/IsUsable.UseItem`
  (params (`AI Character` :type "/Game/Blueprints/AI/AIS_Character Object Reference"))
  (bind _aistatarray (`/Game/Blueprints/AI/AIS_Character.AiStatArray` `AI Character`))
  (bind (_currentstatvalue _minstat _maxstat _statdesirability _statdecayrate _statbehaviors) (break `/Game/Blueprints/AI/DataTable/StatStruct` (`|GetArrayItem` _aistatarray (`self.StatIndex`))))
  (`KismetArrayLibrary.Array_Set` _aistatarray (`self.StatIndex`) (make `/Game/Blueprints/AI/DataTable/StatStruct` (`KismetMathLibrary.FClamp` (+ (`self.StatRestore`) _currentstatvalue) _minstat _maxstat) _minstat _maxstat _statdesirability _statdecayrate _statbehaviors))
  (`self.K2_DestroyActor`))

(fn `UserConstructionScript`)