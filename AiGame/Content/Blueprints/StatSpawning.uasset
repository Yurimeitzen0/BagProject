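; StatSpawning is an actor that periodically spawns Apple stat items around itself.
; On BeginPlay it starts a looping timer and registers itself as a sight stimulus source for AI perception.
; Each tick of the timer spawns an Apple above a random navigable point within the far spawn range, passes it the primary stat index and gives it a random spin.
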(event `self.ReceiveBeginPlay`
  (`KismetSystemLibrary.K2_SetTimerDelegate` (delegate `SpawnStatItem`) (`self.SpawnRate`) true)
  (`AIPerceptionSystem.RegisterPerceptionStimuliSource` "/Script/AIModule.AISense_Sight" self))

(event `SpawnStatItem`
  (bind _returnvalue (`|SpawnActorFromClass` "/Game/Blueprints/Food/Apple.Apple_C" (`KismetMathLibrary.Conv_VectorToTransform` (+ (`NavigationSystemV1.K2_GetRandomLocationInNavigableRadius` (`self.K2_GetActorLocation`) (`self.FarSpawnRange`) null null) (0.0 0.0 150.0))) "Undefined" "OverrideRootScale" null (`self.PrimaryStatIndex`) null))
  (`PrimitiveComponent.SetPhysicsAngularVelocityInDegrees` (`/Game/Blueprints/Food/GoodFood.StaticMesh` _returnvalue) (* (`KismetMathLibrary.RandomUnitVector`) 100.0) false "None"))

(fn `UserConstructionScript`)