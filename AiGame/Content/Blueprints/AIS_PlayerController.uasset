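; Player controller for a free-moving camera pawn that selects IsUsable actors and shows them in a StatBlock HUD.
; Movement axes offset the stored pawn horizontally relative to control rotation.
; Tick-fed gates time mouse presses: a short left click selects via cursor trace, a short right click deselects, and holding right rotates the spring arm and control yaw.
; Tick also aligns pawn yaw and applies mouse-position deltas to control rotation.
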(event `InputAxis|MoveForward`
  (params (AxisValue :type "Float (single-precision)"))
  (bind _returnvalue (`self.GetControlRotation`))
  (`self.K2_AddActorLocalOffset` (`self.StoredPawn`) (* (* (+ (* (`KismetMathLibrary.GetForwardVector` _returnvalue) AxisValue) (* (`KismetMathLibrary.GetRightVector` _returnvalue) (stale `InputAxis|MoveRight` AxisValue))) (`self.MovementRate`)) (1.0 1.0 0.0)) false false :!label _label)
  (`SceneComponent.K2_SetWorldRotation` (`/Game/Blueprints/AIS_PlayerPawn.ControllerArrow` (`self.StoredPawn`)) (`self.GetControlRotation`) false false))

(event `InputAxis|MoveRight`
  (params (AxisValue :type "Float (single-precision)"))
  (goto _label))

(event `Key|LeftMouseButton`
  (params (Key :type "Key Structure"))
  (bind _leftclickholdcounter (`self.LeftClickHoldCounter`))
  (:`Pressed`
    (set `self.bLeftClick` true)
    (goto _label_2 :!via `Open`))
  (:`Released`
    (if (not (not (`self.bLeftClick`)))
      (`self.LeftClickAction`))
    (set `self.LeftClickHoldCounter` 0.0)
    (goto _label_2 :!via `Close`)))

(event `self.ReceiveTick`
  (params (DeltaSeconds :type "Float (single-precision)"))
  (bind (_locationx _locationy) (`self.GetMousePosition`))
  (bind (_locationx_2 _locationy_2) (`self.GetMousePosition`))
  (bind _rightclickholdcounter (`self.RightClickHoldCounter`))
  (bind _leftclickholdcounter (`self.LeftClickHoldCounter`))
  (bind _yaw (.yaw (`self.GetControlRotation`)))
  (bind _springarm (`/Game/Blueprints/AIS_PlayerPawn.SpringArm` (`self.StoredPawn`)))
  (`|ExecutionSequence`
    (:`then_0`
      (`/Engine/EditorBlueprintResources/StandardMacros.Gate` true :!label _label_2
        (:`Exit`
          (if (`self.bLeftClick`)
            (if (>= _leftclickholdcounter 0.06)
              (set `self.bLeftClick` false)
              (else
                (set `self.LeftClickHoldCounter` (+ DeltaSeconds _leftclickholdcounter))))))))
    (:`then_1`
      (`/Engine/EditorBlueprintResources/StandardMacros.Gate` true :!label _label_3
        (:`Exit`
          (if (`self.bRightClick`)
            (if (>= _rightclickholdcounter 0.06)
              (set `self.bRightClick` false)
              (else
                (set `self.RightClickHoldCounter` (+ DeltaSeconds _rightclickholdcounter))))
            (else
              (`self.SetControlRotation` (`KismetMathLibrary.MakeRotator` 0.0 0.0 (+ (`self.GetInputAxisKeyValue`) (.yaw (`self.GetControlRotation`)))))
              (`SceneComponent.K2_SetWorldRotation` _springarm (`KismetMathLibrary.MakeRotator` 0.0 (+ (`self.GetInputAxisKeyValue`) (.pitch (`SceneComponent.K2_GetComponentRotation` _springarm))) (+ (`self.GetInputAxisKeyValue`) (.yaw (`SceneComponent.K2_GetComponentRotation` _springarm)))) false false))))))
    (:`then_2`
      (set `self.PreviousX` _locationx_2)
      (set `self.PreviousY` _locationy_2)
      (`self.K2_SetActorRotation` (`self.StoredPawn`) (`KismetMathLibrary.MakeRotator` 0.0 0.0 _yaw) false)
      (`self.SetControlRotation` (`KismetMathLibrary.MakeRotator` (.roll (`self.GetControlRotation`)) (+ (.pitch (`self.GetControlRotation`)) (* (* (- _locationy (`self.PreviousY`)) 0.07) 4.0)) (+ _yaw (* (* (- _locationx (`self.PreviousX`)) 0.07) 4.0)))))))

(event `Key|RightMouseButton`
  (params (Key :type "Key Structure"))
  (:`Pressed`
    (set `self.bRightClick` true)
    (goto _label_3 :!via `Open`))
  (:`Released`
    (if (not (not (`self.bRightClick`)))
      (`self.RightClickAction`))
    (set `self.RightClickHoldCounter` 0.0)
    (goto _label_3 :!via `Close`)))

(event `LeftClickAction`
  (bind _selectedthing (`self.SelectedThing`))
  (bind (_bblockinghit _binitialoverlap _time _distance _location _impactpoint _normal _impactnormal _physmat _hitactor) (`GameplayStatics.BreakHitResult` (`self.GetHitResultUnderCursorByChannel` "TraceTypeQuery2")))
  (bind _asstat_block (cast `/Game/UI/StatBlock` (`WidgetComponent.GetUserWidgetObject` (`/Game/Blueprints/AIS_PlayerPawn.HUD` (`self.StoredPawn`))) :!pure true))
  (if (`KismetSystemLibrary.DoesImplementInterface` _hitactor "/Game/Interfaces/IsUsable.IsUsable_C")
    (`KismetSystemLibrary.PrintString` (`KismetSystemLibrary.GetDisplayName` _hitactor))
    (`/Engine/EditorBlueprintResources/StandardMacros.IsValid` _selectedthing
      (:`Is Valid`
        (message `/Game/Interfaces/IsUsable.Deselected` _selectedthing))
      (:`Is Not Valid`
        _))
    (bind _output_get (set `self.SelectedThing` _hitactor))
    (message `/Game/Interfaces/IsUsable.Selected` _output_get)
    (set `/Game/UI/StatBlock.OwningPawn` (cast `/Game/Blueprints/AI/AIS_Character` _output_get :!pure true) _asstat_block)
    (`/Game/UI/StatBlock.UpdateHUD` _asstat_block)
    (`Widget.SetVisibility` _asstat_block "Visible")))

(event `RightClickAction`
  (bind _selectedthing (`self.SelectedThing`))
  (bind _returnvalue (`WidgetComponent.GetUserWidgetObject` (`/Game/Blueprints/AIS_PlayerPawn.HUD` (`self.StoredPawn`))))
  (`/Engine/EditorBlueprintResources/StandardMacros.IsValid` _selectedthing
    (:`Is Valid`
      (message `/Game/Interfaces/IsUsable.Deselected` _selectedthing)
      (set `self.SelectedThing` null)
      (`Widget.SetVisibility` _returnvalue "Hidden")
      (bind _asstat_block (cast `/Game/UI/StatBlock` _returnvalue))
      (`/Game/UI/StatBlock.ClearPawn` _asstat_block))))

(fn `UserConstructionScript`)