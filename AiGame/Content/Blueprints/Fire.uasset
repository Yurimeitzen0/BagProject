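; Short-lived fire hazard actor that damages AI characters on contact.
; On BeginPlay it waits through a fixed delay, then deactivates its particle and destroys itself.
; Capsule overlaps with IsUsable implementers are cast to AIS_Character and passed to DoFireDamage.
; That event lowers the character's first AI stat once by that stat's own decay rate, clamped to its limits, rather than using a separate damage value.
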(event `self.ReceiveBeginPlay`
  (`KismetSystemLibrary.Delay` 10.0)
  (`ActorComponent.Deactivate` (`self.FireParticle`))
  (`self.K2_DestroyActor`))

(event `/Game/Interfaces/IsUsable.DoFireDamage`
  (params (AiCharacter :type "/Game/Blueprints/AI/AIS_Character Object Reference"))
  (bind _aistatarray (`/Game/Blueprints/AI/AIS_Character.AiStatArray` AiCharacter))
  (bind (_currentstatvalue _minstat _maxstat _statdesirability _statdecayrate _statbehaviors) (break `/Game/Blueprints/AI/DataTable/StatStruct` (`|GetArrayItem` _aistatarray)))
  (`/Engine/EditorBlueprintResources/StandardMacros.IsValid` AiCharacter
    (:`Is Valid`
      (`KismetArrayLibrary.Array_Set` _aistatarray 0 (make `/Game/Blueprints/AI/DataTable/StatStruct` (`KismetMathLibrary.FClamp` (- _currentstatvalue _statdecayrate) _minstat _maxstat) _minstat _maxstat _statdesirability _statdecayrate _statbehaviors)))))

(event `self.CapsuleCollider.OnComponentBeginOverlap`
  (params (OverlappedComponent :type "PrimitiveComponent Object Reference") (OtherActor :type "Actor Object Reference") (OtherComp :type "PrimitiveComponent Object Reference") (OtherBodyIndex :type Integer) (bFromSweep :type Boolean) (SweepResult :type "HitResult Structure (by ref)"))
  (if (`KismetSystemLibrary.DoesImplementInterface` OtherActor "/Game/Interfaces/IsUsable.IsUsable_C")
    (`/Game/Interfaces/IsUsable.DoFireDamage` (cast `/Game/Blueprints/AI/AIS_Character` OtherActor :!pure true))))

(fn `UserConstructionScript`)