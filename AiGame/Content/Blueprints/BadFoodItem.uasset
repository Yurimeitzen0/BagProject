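; BadFoodItem is a usable item that harms the AI character who consumes it.
; On BeginPlay it sets its StatRestore amount before calling the parent.
; UseItem applies DamageToApply to that character, with the item as damage causer, then passes to the parent's UseItem logic.
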(event `self.ReceiveBeginPlay`
  (set `self.StatRestore` 100.0)
  (`parent.ReceiveBeginPlay`))

(event `/Game/Interfaces/IsUsable.UseItem`
  (params (`AI Character` :type "/Game/Blueprints/AI/AIS_Character Object Reference"))
  (`GameplayStatics.ApplyDamage` `AI Character` (`self.DamageToApply`) null self)
  (`parent.UseItem` `AI Character`))

(fn `UserConstructionScript`
  (`parent.UserConstructionScript`))