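; GoodFood is a consumable food item that adjusts an AI character's stats when used and registers itself as a sight perception stimulus.
; UseItem adds StatRestore values to the character's stats from index 1 onward, clamped to each stat's limits.
; Index 0 is handled separately: a zero or negative value is applied as damage, while a positive one has no effect.
; PostUse then destroys the actor after a brief delay.
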(event `self.ReceiveBeginPlay`
  ;[1 1 1] Optional?
  (`AIPerceptionSystem.RegisterPerceptionStimuliSource` "/Script/AIModule.AISense_Sight" self))

(event `/Game/Interfaces/IsUsable.UseItem`
  (params (`AI Character` :type "/Game/Blueprints/AI/AIS_Character Object Reference"))
  (bind _aistatarray (`/Game/Blueprints/AI/AIS_Character.AiStatArray` `AI Character`))
  (bind _output (`|GetArrayItem` (`self.StatRestore`)))
  (for _index (range 1 (+ (`KismetArrayLibrary.Array_LastIndex` _aistatarray) 1))
    (bind (_currentstatvalue _minstat _maxstat _statdesirability _statdecayrate _statbehaviors) (break `/Game/Blueprints/AI/DataTable/StatStruct` (`|GetArrayItem` _aistatarray _index)))
    (`KismetArrayLibrary.Array_Set` _aistatarray _index (make `/Game/Blueprints/AI/DataTable/StatStruct` (`KismetMathLibrary.FClamp` (+ (`|GetArrayItem` (`self.StatRestore`) _index) _currentstatvalue) _minstat _maxstat) _minstat _maxstat _statdesirability _statdecayrate _statbehaviors)))
  (if (<= _output 0.0)
    (`GameplayStatics.ApplyDamage` `AI Character` (`KismetMathLibrary.Abs` _output) null self))
  (`self.Post Use`))

(event `Post Use`
  (`KismetSystemLibrary.Delay` 0.1)
  (`self.K2_DestroyActor`))

(fn `UserConstructionScript`)