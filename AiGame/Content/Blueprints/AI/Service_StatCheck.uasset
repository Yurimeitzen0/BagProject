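; Behavior Tree service that checks an AI character's stats and flags when one is depleted enough to act on.
; Each tick it uses the cached AIS_Character pawn and converts every AiStatArray entry into a percentage depleted from max toward min.
; The most depleted stat at or above StatThreshold has its index written to DesiredStatKey.
; FindFoodKey records whether any stat qualified, whichever stat it was.
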(event EventReceiveTickAI
  (params (OwnerController :type AI%20Controller%20Object%20Reference) (ControlledPawn :type Pawn%20Object%20Reference) (DeltaSeconds :type Float%20%28single-precision%29))
  (Variables|Default|SetPossibilyFoundStat false)
  (Utilities|IsValid (Variables|Default|GetAiPawn)
    (:Is%20Valid
      _)
    (:Is%20Not%20Valid
      (bind _asais_character (Utilities|Casting|CastToAIS_Character ControlledPawn))
      (Variables|Default|SetAiPawn _asais_character)))
  (Variables|Default|SetTestValue 0.0)
  (for (_array_element _array_index) (Variables|/Game/Blueprints/AI/AIS_Character.AIS_Character_C|GetAiStatArray (Variables|Default|GetAiPawn))
    (if (>= (* (|(1-((Current-Min)/(Max-Min))) (.CurrentStatValue (Utilities|Struct|BreakStatStruct _array_element)) (.MinStat (Utilities|Struct|BreakStatStruct _array_element)) (.MaxStat (Utilities|Struct|BreakStatStruct _array_element))) 1e+02) (Variables|Default|GetStatThreshold))
      (Variables|Default|SetPossibilyFoundStat true)
      (if (> (* (|(1-((Current-Min)/(Max-Min))) (.CurrentStatValue (Utilities|Struct|BreakStatStruct _array_element)) (.MinStat (Utilities|Struct|BreakStatStruct _array_element)) (.MaxStat (Utilities|Struct|BreakStatStruct _array_element))) 1e+02) (Variables|Default|GetTestValue))
        (bind _output_get (Variables|Default|SetChosenStat _array_index))
        (Variables|Default|SetTestValue (* (|(1-((Current-Min)/(Max-Min))) (.CurrentStatValue (Utilities|Struct|BreakStatStruct _array_element)) (.MinStat (Utilities|Struct|BreakStatStruct _array_element)) (.MaxStat (Utilities|Struct|BreakStatStruct _array_element))) 1e+02))
        (Development|PrintString (Utilities|String|ToString(Integer) _output_get)))))
  (if (Variables|Default|GetPossibilyFoundStat)
    (Class|BTFunctionLibrary|SetBlackboardValueasInt (Variables|Default|GetDesiredStatKey) (Variables|Default|GetChosenStat))
    (Class|BTFunctionLibrary|SetBlackboardValueasBool (Variables|Default|GetFindFoodKey) true)
    (else
      (Class|BTFunctionLibrary|SetBlackboardValueasBool (Variables|Default|GetFindFoodKey) false))))