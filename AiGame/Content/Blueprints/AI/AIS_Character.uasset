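; AI character with data-driven survival stats, built from StatTable at BeginPlay with optional per-instance starting values; row names are shared through AIS_GameState.
; A looping timer drains hunger (stat 2), then stat 1 once hunger empties, regenerating health (stat 0) until both are empty, then applying damage.
; Damage lowers health and destroys the character at zero.
; Events also handle dialogue callouts, montage forwarding and interface-based item use.
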(event `DialogCallout`
  (params (ThingToTalkAbout :type "Actor Object Reference"))
  (bind _mesh (`self.Mesh`))
  ;[1 1 1] Dialogue Handler For Identifying object
  (`GameplayStatics.SpawnDialogueAttached` "/Game/Blueprints/Audio/IFound_Gender.IFound_Gender" (make `DialogueContext` (`|GetArrayItem` (`/Game/Blueprints/DialogComponent.DialogContext` (`self.DialogComponent`))) (`/Game/Blueprints/DialogComponent.DialogContext` (`self.GetComponentByClass` ThingToTalkAbout "/Game/Blueprints/DialogComponent.DialogComponent_C"))) _mesh "head" (`SceneComponent.K2_GetComponentLocation` _mesh)))

(event `self.ReceiveBeginPlay`
  (bind _currentstatvalue (`self.CurrentStatValue`))
  (`KismetSystemLibrary.K2_SetTimerDelegate` (delegate `Starve`) (`self.StatTickRate`) true) ; Custom Tick for stamina consumption
  (bind _asais_game_state (cast `/Game/Blueprints/AIS_GameState` (`GameplayStatics.GetGameState`))
    (:`then`
      (bind _output_get (set `self.StoredGameState` _asais_game_state))
      (bind _outrownames (`DataTableFunctionLibrary.GetDataTableRowNames` "/Game/Blueprints/AI/DataTable/StatTable.StatTable"))
      (bind _output_get_2 (set `/Game/Blueprints/AIS_GameState.StatNames` _outrownames _output_get))
      (for (_array_element _array_index) _output_get_2
        (bind _returnvalue (`|GetDataTableRow` "/Game/Blueprints/AI/DataTable/StatTable.StatTable" _array_element)
          (:`then`
            (bind (_currentstatvalue_2 _minstat _maxstat _statdesirability _statdecayrate _statbehaviors) (break `/Game/Blueprints/AI/DataTable/StatStruct` _returnvalue))
            (bind _output (`|GetArrayItem` _currentstatvalue _array_index))
            (`KismetArrayLibrary.Array_AddUnique` (`self.AiStatArray`) (make `/Game/Blueprints/AI/DataTable/StatStruct` (`KismetMathLibrary.SelectFloat` _currentstatvalue_2 _output (or (<= _output 0.0) (> _array_index (`KismetArrayLibrary.Array_LastIndex` _currentstatvalue)))) _minstat _maxstat _statdesirability _statdecayrate _statbehaviors))))))
    (:`CastFailed`
      (`KismetSystemLibrary.PrintString` "CARALHO"))))

(event `Starve`
  (bind (_currentstatvalue _minstat _maxstat _statdesirability _statdecayrate _statbehaviors) (break `/Game/Blueprints/AI/DataTable/StatStruct` (`|GetArrayItem` (`self.AiStatArray`))))
  (`self.StatTickDown` 2) ; Ticks Hunger(stat 2)
  (if (<= (`.CurrentStatValue_5_1454EF404CC5F130DB9F63BF17BFCBCA` (break `/Game/Blueprints/AI/DataTable/StatStruct` (`|GetArrayItem` (`self.AiStatArray`) 2))) 0.0)
    (`self.StatTickDown` 1)
    (if (<= (`.CurrentStatValue_5_1454EF404CC5F130DB9F63BF17BFCBCA` (break `/Game/Blueprints/AI/DataTable/StatStruct` (`|GetArrayItem` (`self.AiStatArray`) 1))) 0.0)
      (`GameplayStatics.ApplyDamage` self 5.0 null self)
      (else
        (`KismetArrayLibrary.Array_Set` (`self.AiStatArray`) 0 (make `/Game/Blueprints/AI/DataTable/StatStruct` (`KismetMathLibrary.FClamp` (+ _currentstatvalue _statdecayrate) _minstat _maxstat) _minstat _maxstat _statdesirability _statdecayrate _statbehaviors))))))

(event `/Game/Interfaces/AIAnimation.ControllerToCharacter`
  (params (MontageIndex :type Integer))
  (message `/Game/Interfaces/AIAnimation.CharacterToAnimBP` (`SkeletalMeshComponent.GetAnimInstance` (`self.Mesh`)) MontageIndex))

(event `self.ReceiveAnyDamage`
  (params (Damage :type "Float (single-precision)") (DamageType :type "DamageType Object Reference") (InstigatedBy :type "Controller Object Reference") (DamageCauser :type "Actor Object Reference"))
  (bind (_currentstatvalue _minstat _maxstat _statdesirability _statdecayrate _statbehaviors) (break `/Game/Blueprints/AI/DataTable/StatStruct` (`|GetArrayItem` (`self.AiStatArray`))))
  (bind _returnvalue (`KismetMathLibrary.FClamp` (- _currentstatvalue Damage) _minstat _maxstat))
  ;[1 1 1] Handles damage logic
  (`KismetSystemLibrary.PrintString` "Feeling like a true communist!!!")
  (`KismetArrayLibrary.Array_Set` (`self.AiStatArray`) 0 (make `/Game/Blueprints/AI/DataTable/StatStruct` _returnvalue _minstat _maxstat _statdesirability _statdecayrate _statbehaviors))
  (if (<= _returnvalue 0.0)
    (`Controller.UnPossess` (`self.GetController`))
    (`self.K2_DestroyActor`)))

(event `/Game/Interfaces/IsUsable.AiUseItem`
  (params (ItemToUse :type "Actor Object Reference"))
  ;[1 1 1] Using item with the desired interface
  (if (`KismetSystemLibrary.DoesImplementInterface` ItemToUse "/Game/Interfaces/IsUsable.IsUsable_C")
    (message `/Game/Interfaces/IsUsable.UseItem` ItemToUse self)
    (else
      (`KismetSystemLibrary.PrintString` "Unusable Item"))))

(fn `StatTickDown`
  (params (StatToTick :type Integer))
  (bind (_currentstatvalue _minstat _maxstat _statdesirability _statdecayrate _statbehaviors) (break `/Game/Blueprints/AI/DataTable/StatStruct` (`|GetArrayItem` (`self.AiStatArray`) StatToTick)))
  (`KismetArrayLibrary.Array_Set` (`self.AiStatArray`) StatToTick (make `/Game/Blueprints/AI/DataTable/StatStruct` (`KismetMathLibrary.FClamp` (- _currentstatvalue (* _statdecayrate (`self.StatTickRate`))) _minstat _maxstat) _minstat _maxstat _statdesirability _statdecayrate _statbehaviors)))

(fn `UserConstructionScript`)