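; AI controller that runs the AIS_BT behavior tree on BeginPlay and carries an AIPerception component.
; Target perception updates only print the actor's name and stimulus age as debug output, with nothing passed to the tree in this graph.
; The OnPerceptionUpdated handler is empty, and a loop that prints updated actor names sits disconnected.
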(event `self.AIPerception.OnPerceptionUpdated`
  (params (UpdatedActors :type "Array of Actor Object Reference")))

(event `self.AIPerception.OnTargetPerceptionUpdated`
  (params (Actor :type "Actor Object Reference") (Stimulus :type "AIStimulus Structure"))
  (`KismetSystemLibrary.PrintString` (`KismetStringLibrary.Concat_StrStr` (`KismetSystemLibrary.GetDisplayName` Actor) "Age: " (`KismetStringLibrary.Conv_DoubleToString` (`.Age` (break `AIStimulus` Stimulus))))))

(event `self.ReceiveBeginPlay`
  (`self.RunBehaviorTree` "/Game/Blueprints/AI/AIS_BT.AIS_BT"))

(fn `UserConstructionScript`)