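; Behavior tree service that flags whether the AI currently sees a harmful object, treated as fire.
; On each tick it looks up every entry of the AIS_AiCon controller's HarmfulObjects among sight-perceived actors and writes the FireSpotted blackboard bool.
; Each entry overwrites the flag, so the last one decides the result.
; The Find > 0 test ignores a match at index 0.
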(event `self.ReceiveTickAI`
  (params (OwnerController :type "AIController Object Reference") (ControlledPawn :type "Pawn Object Reference") (DeltaSeconds :type "Float (single-precision)"))
  (set `self.FireFound` false)
  (for _array_element (`/Game/Blueprints/AI/AIS_AiCon.HarmfulObjects` (cast `/Game/Blueprints/AI/AIS_AiCon` OwnerController :!pure true))
    (if (> (`KismetArrayLibrary.Array_Find` (`AIPerceptionComponent.GetPerceivedActors` (`AIController.GetAIPerceptionComponent` OwnerController) "/Script/AIModule.AISense_Sight") _array_element) 0)
      (`KismetSystemLibrary.PrintString` "FireFound")
      (set `self.FireFound` true)
      (`BTFunctionLibrary.SetBlackboardValueAsBool` (`self.FireSpotted`) (`self.FireFound`))
      (else
        (bind _output_get (set `self.FireFound` false))
        (`BTFunctionLibrary.SetBlackboardValueAsBool` (`self.FireSpotted`) _output_get)))))