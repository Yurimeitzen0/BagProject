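; GoodFood is a consumable item that restores one stat on the AI character that uses it.
; UseItem adds StatRestore to the character's CurrentStatValue entry at StatIndex, clamps the result to that stat's StatMin and StatMax, then destroys the item.
; The affected stat is selected by array index, so the logic is not tied to a named stat.
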(event `/Game/Interfaces/IsUsable.UseItem`
  (params (`AI Character` :type "/Game/Blueprints/AI/AIS_Character Object Reference"))
  (bind _currentstatvalue (`/Game/Blueprints/AI/AIS_Character.CurrentStatValue` `AI Character`))
  (bind _statindex (`self.StatIndex`))
  (`KismetArrayLibrary.Array_Set` _currentstatvalue (`self.StatIndex`) (`KismetMathLibrary.FClamp` (+ (`|GetArrayItem` _currentstatvalue _statindex) (`self.StatRestore`)) (`|GetArrayItem` (`/Game/Blueprints/AI/AIS_Character.StatMin` `AI Character`) _statindex) (`|GetArrayItem` (`/Game/Blueprints/AI/AIS_Character.StatMax` `AI Character`) _statindex)))
  (`self.K2_DestroyActor`))

(fn `UserConstructionScript`)